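; BP_TeleportPad is a pad that teleports the third-person character to a linked pad.
; On BeginPlay it finds pads by the LinkedPad tag and uses the first as its destination.
; Box overlap flags that destination as just triggered, waits briefly, then moves the player above it.
; JustTriggered blocks an immediate bounce back, and EventLocked, released after teleport, lets the destination's end overlap re-arm it.
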(event `self.ReceiveBeginPlay`
  (bind _outactors (`GameplayStatics.GetAllActorsOfClassWithTag` "BP_TeleportPad_C" (`self.LinkedPad`)))
  (set `self.PadArray` _outactors))

(event `self.BoxCollision.OnComponentBeginOverlap`
  (params (OverlappedComponent :type "PrimitiveComponent Object Reference") (OtherActor :type "Actor Object Reference") (OtherComp :type "PrimitiveComponent Object Reference") (OtherBodyIndex :type Integer) (bFromSweep :type Boolean) (SweepResult :type "HitResult Structure (by ref)"))
  (bind _output (`|GetArrayItem` (`self.PadArray`)))
  (bind _asbp_third_person_character (cast `/Game/ThirdPerson/Blueprints/BP_ThirdPersonCharacter` OtherActor))
  (set `self.PlayerRef` _asbp_third_person_character)
  (if (not (`self.JustTriggered`))
    (`/Engine/EditorBlueprintResources/StandardMacros.IsValid` _output
      (:`Is Valid`
        (set `/Game/Blueprints/BP_TeleportPad.JustTriggered` true _output)
        (`KismetSystemLibrary.Delay` 0.5)
        (`self.K2_SetActorRelativeLocation` (`self.PlayerRef`) (+ (`SceneComponent.RelativeLocation` (`/Game/Blueprints/BP_TeleportPad.DefaultSceneRoot` _output)) (0.0 0.0 100.0)) false false)
        (set `/Game/Blueprints/BP_TeleportPad.EventLocked` false _output)))))

(event `self.BoxCollision.OnComponentEndOverlap`
  (params (OverlappedComponent :type "PrimitiveComponent Object Reference") (OtherActor :type "Actor Object Reference") (OtherComp :type "PrimitiveComponent Object Reference") (OtherBodyIndex :type Integer))
  (if (not (`self.EventLocked`))
    (set `self.JustTriggered` false)
    (set `self.EventLocked` true)))

(fn `UserConstructionScript`)